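; LaserEmisor is a laser hazard actor that damages the first-person character crossing the line between it and its paired LaserReceptor.
; Every Tick it traces from its Sphere to the receptor's root for Pawn objects, drawing the trace as a one-frame debug line.
; A FirstPersonCharacter hit takes Damage each frame, unscaled by delta time, and its CurrentLife is printed on screen.
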(event EventBeginPlay)

(event Collision|EventActorBeginOverlap
  (params (OtherActor :type Actor%20Object%20Reference)))

(event EventTick
  (params (DeltaSeconds :type Float%20%28single-precision%29))
  (bind _outhit (Collision|LineTraceForObjects (Transformation|GetWorldLocation (Variables|Default|GetSphere)) (Transformation|GetWorldLocation (Variables|/Script/Engine.Actor|GetRootComponent (Variables|Default|GetLaserReceptor))) (Utilities|Array|MakeArray "ObjectTypeQuery3") false 0 "ForOneFrame"))
  (Utilities|IsValid (.HitActor (Collision|BreakHitResult _outhit))
    (:Is%20Valid
      (bind _asfirst_person_character (Utilities|Casting|CastToFirstPersonCharacter (.HitActor (Collision|BreakHitResult _outhit))))
      (Default|ApplyDamagetoCharacter _asfirst_person_character (Variables|Default|GetDamage))
      (Development|PrintString (Utilities|String|ToString(Integer) (Variables|/Game/FirstPersonBP/Blueprints/FirstPersonCharacter.FirstPersonCharacter_C|GetCurrentLife _asfirst_person_character))))))

(fn ConstructionScript)